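; BP_Collectible is a pickup actor that the player character collects on touch.
; On BeginPlay the Spin timeline animates the small pine tree mesh, remapping its Bounce and SpinAmount tracks to relative height and yaw.
; A BP_Character entering DetectionZone triggers a DoOnce that increments that character's Collected count, prints a message and destroys the actor after a short delay.
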(event OnComponentBeginOverlap(detectionzone)
  (params (OverlappedComponent :type Primitive%20Component%20Object%20Reference) (OtherActor :type Actor%20Object%20Reference) (OtherComp :type Primitive%20Component%20Object%20Reference) (OtherBodyIndex :type Integer) (bFromSweep :type Boolean) (SweepResult :type Hit%20Result%20Structure%20%28by%20ref%29))
  (bind _asbp_character (Utilities|Casting|CastToBP_Character OtherActor))
  (Utilities|FlowControl|DoOnce false
    (:Completed
      (Math|Integer|IncrementInt (Variables|/Game/BP/GameDefaults/BP_Character.BP_Character_C|Getcollected _asbp_character)
        (:%20%20
          (Development|PrintString "Collected!")
          (Utilities|FlowControl|Delay 0.2)
          (Actor|DestroyActor))))))

(event EventBeginPlay
  (bind (_direction _spin_amount _bounce) (Timeline|Spin Play)
    (:Update
      (Transformation|SetRelativeLocationAndRotation (Variables|Default|Gettree-pine-small) (Math|Vector|MakeVector 0.0 0.0 (Math|Float|MapRangeClamped _bounce 0.0 1.0 0.0 5e+01)) (Math|Rotator|MakeRotator 0.0 0.0 (Math|Float|MapRangeClamped _spin_amount 0.0 1.0 0.0 7.2e+02)) false false))))

(fn ConstructionScript)