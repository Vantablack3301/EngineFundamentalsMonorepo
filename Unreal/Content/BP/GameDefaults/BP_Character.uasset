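; BP_Character is the player character, with Enhanced Input actions for walking, looking, jumping and attacking.
; On BeginPlay it registers itself as Player on BP_GameMode, then creates the W_Hud widget and adds it to the player screen.
; The attack restarts a timeline that spins the static mesh through two full yaw turns while repeatedly launching the character forward on every update.
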(event Input|EnhancedActionEvents|EnhancedInputActionIA_Walking
  (params (ActionValue :type Vector%202D%20Structure) (ElapsedSeconds :type Float%20%28double-precision%29) (TriggeredSeconds :type Float%20%28double-precision%29) (InputAction :type Input%20Action%20Object%20Reference :default "/Game/BP/input/IA_Walking.IA_Walking"))
  (Pawn|Input|AddMovementInput (Transformation|GetActorForwardVector) (.x ActionValue) false)
  (Pawn|Input|AddMovementInput (Transformation|GetActorRightVector) (.y ActionValue) false))

(event Input|EnhancedActionEvents|EnhancedInputActionIA_Look
  (params (ActionValue :type Vector%202D%20Structure) (ElapsedSeconds :type Float%20%28double-precision%29) (TriggeredSeconds :type Float%20%28double-precision%29) (InputAction :type Input%20Action%20Object%20Reference :default "/Game/BP/input/IA_Look.IA_Look"))
  (Pawn|Input|AddControllerPitchInput (* (.y ActionValue) -1.0))
  (Pawn|Input|AddControllerYawInput (.x ActionValue)))

(event Input|EnhancedActionEvents|EnhancedInputActionIA_Jump
  (params (ActionValue :type Boolean) (ElapsedSeconds :type Float%20%28double-precision%29) (TriggeredSeconds :type Float%20%28double-precision%29) (InputAction :type Input%20Action%20Object%20Reference :default "/Game/BP/input/IA_Jump.IA_Jump"))
  (Character|Jump))

(event Input|EnhancedActionEvents|EnhancedInputActionIA_Attack
  (params (ActionValue :type Boolean) (ElapsedSeconds :type Float%20%28double-precision%29) (TriggeredSeconds :type Float%20%28double-precision%29) (InputAction :type Input%20Action%20Object%20Reference :default "/Game/BP/input/IA_Attack.IA_Attack"))
  (bind _spin (Timeline|Timeline PlayFromStart)
    (:Update
      (Transformation|SetRelativeRotation (Variables|Default|GetStaticMesh) (Math|Rotator|MakeRotator 0.0 0.0 (Math|Float|MapRangeClamped _spin 0.0 1.0 0.0 7.2e+02)) false false)
      (Character|LaunchCharacter (* (Transformation|GetActorForwardVector) 5e+02) false false))))

(event EventBeginPlay
  (bind _asbp_game_mode (Utilities|Casting|CastToBP_GameMode (Game|GetGameMode)))
  (Variables|/Game/BP/GameDefaults/BP_GameMode.BP_GameMode_C|SetPlayer _asbp_game_mode self)
  (bind _returnvalue (UserInterface|CreateWidget "/Game/BP/GameDefaults/W_Hud.W_Hud_C" (Pawn|GetLocalViewingPlayerController self)))
  (UserInterface|Viewport|AddtoPlayerScreen _returnvalue))

(fn ConstructionScript)